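; DepthAffectedWalls_BP is a wall mesh actor that shows or hides itself according to the player's depth along the world X axis.
; Every tick it compares its X location with that of player character 0, hiding the StaticMeshComponent in game when the wall's X is greater and showing it otherwise.
; The check only toggles visibility, without propagating to child components or changing collision settings.
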(event `self.ReceiveTick`
  (params (DeltaSeconds :type "Float (single-precision)"))
  (bind _returnvalue_x (`KismetMathLibrary.BreakVector` (`self.K2_GetActorLocation`)))
  (bind _staticmeshcomponent (`self.StaticMeshComponent`))
  (bind _returnvalue_x_2 (`KismetMathLibrary.BreakVector` (`self.K2_GetActorLocation` (`GameplayStatics.GetPlayerCharacter` 0))))
  (`parent.ReceiveTick` DeltaSeconds)
  (if (> _returnvalue_x _returnvalue_x_2)
    (`SceneComponent.SetHiddenInGame` _staticmeshcomponent true false)
    (else
      (`SceneComponent.SetHiddenInGame` _staticmeshcomponent false false))))

(fn `UserConstructionScript`
  (`parent.UserConstructionScript`))