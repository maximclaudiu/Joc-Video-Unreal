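; Base quest actor that tracks objective progress for the current stage of a data-table-driven quest.
; On BeginPlay it loads its QuestID row, zeroes a per-objective progress map and binds to the player SideScrollerCharacter's objective ID event.
; OnObjectiveIDHeard increments matching progress up to the required quantity.
; FinishStage, uncalled here, advances and reloads the stage, though its check passes while progress is at or below quantity.
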(event `self.ReceiveBeginPlay`
  (`self.GetQuestDetails`)
  (add `/Game/Blueprints/Third_person/SideScrollerCharacter.OnObjectiveIDCalled` (cast `/Game/Blueprints/Third_person/SideScrollerCharacter` (`GameplayStatics.GetPlayerCharacter` 0) :!pure true) (`|CreateDelegate` :!event `On Objective ID Heard`)))

(fn `FinishStage`
  (for _array_element (`.Objectives_15_36E4FC594B4E68C4F46A388DBAFA5CBA` (break `/Game/Blueprints/Quests/FStageDetails` (`self.CurrentStageDetails`)))
    (bind (_objectivename _description _type _objectiveid _quantity) (break `/Game/Blueprints/Quests/FObjectiveDetails` _array_element))
    (if (not (>= _quantity (`BlueprintMapLibrary.Map_Find` (`self.CurrentObjectiveProgres`) _objectiveid)))
      (return)))
  (if true
    (`/Engine/EditorBlueprintResources/StandardMacros.IncrementInt` (`self.CurrentStage`)
      (:`  `
        (`self.GetQuestDetails`)))))

(fn `GetQuestDetails`
  (bind _returnvalue (`|GetDataTableRow` "/Game/Blueprints/Quests/QuestDataTable.QuestDataTable" (`self.QuestID`))
    (:`then`
      (bind _output_get (set `self.QuestDetails` _returnvalue))
      (bind _output_get_2 (set `self.CurrentStageDetails` (`|GetArrayItem` (`.Stages_13_D855EC724DC9CAAB44A12DB6028C1A32` (break `/Game/Blueprints/Quests/FQuestDetails` _output_get)) (`self.CurrentStage`))))
      (`BlueprintMapLibrary.Map_Clear` (`self.CurrentObjectiveProgres`))
      (for _array_element (`.Objectives_15_36E4FC594B4E68C4F46A388DBAFA5CBA` (break `/Game/Blueprints/Quests/FStageDetails` _output_get_2))
        (`BlueprintMapLibrary.Map_Add` (`self.CurrentObjectiveProgres`) (`.ObjectiveID_10_C39D87C94F6BABDE3D905581DB53E752` (break `/Game/Blueprints/Quests/FObjectiveDetails` _array_element)))))))

(fn `On Objective ID Heard`
  (params (ObjectiveID :type String))
  (bind (_value _returnvalue) (`BlueprintMapLibrary.Map_Find` (`self.CurrentObjectiveProgres`) ObjectiveID))
  (if _returnvalue
    (for _array_element (`.Objectives_15_36E4FC594B4E68C4F46A388DBAFA5CBA` (break `/Game/Blueprints/Quests/FStageDetails` (`self.CurrentStageDetails`)))
      (bind ((`ObjectiveID_10_C39D87C94F6BABDE3D905581DB53E752` _objectiveid) (`Quantity_13_9F4B78384FC14DE18F7CB7916281DD44` _quantity)) (break `/Game/Blueprints/Quests/FObjectiveDetails` _array_element))
      (if (`KismetStringLibrary.EqualEqual_StrStr` _objectiveid (`local.ObjectiveID`))
        (if (< _value _quantity)
          (`BlueprintMapLibrary.Map_Add` (`self.CurrentObjectiveProgres`) (`local.ObjectiveID`) (+ _value 1))
          (return))))
    (else
      (return))))

(fn `UserConstructionScript`)