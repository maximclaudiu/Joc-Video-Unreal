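; GI_Rush, apparently the game instance, holds a snapshot of the side-scroller player's progress.
; SavePlayerInfo casts player 0's character to SideScrollerCharacter and copies its vitals, coins, level and experience, potions, attributes and unspent points into its own variables.
; It also records the current date and level name; nothing here writes to disk or restores the values.
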(fn `SavePlayerInfo`
  (bind _asside_scroller_character (cast `/Game/Blueprints/Third_person/SideScrollerCharacter` (`GameplayStatics.GetPlayerCharacter` 0)))
  (set `self.Mana` (`/Game/Blueprints/Third_person/SideScrollerCharacter.Mana` _asside_scroller_character))
  (set `self.HP` (`/Game/Blueprints/Third_person/SideScrollerCharacter.HP` _asside_scroller_character))
  (set `self.Coins` (`/Game/Blueprints/Third_person/SideScrollerCharacter.Coins` _asside_scroller_character))
  (set `self.Level` (`/Game/Blueprints/Third_person/SideScrollerCharacter.Level` _asside_scroller_character))
  (set `self.Experience` (`/Game/Blueprints/Third_person/SideScrollerCharacter.Experience` _asside_scroller_character))
  (set `self.ManaPot` (`/Game/Blueprints/Third_person/SideScrollerCharacter.ManaPot` _asside_scroller_character))
  (set `self.HPPot` (`/Game/Blueprints/Third_person/SideScrollerCharacter.HPPot` _asside_scroller_character))
  (set `self.STR` (`/Game/Blueprints/Third_person/SideScrollerCharacter.STR` _asside_scroller_character))
  (set `self.INT` (`/Game/Blueprints/Third_person/SideScrollerCharacter.INT` _asside_scroller_character))
  (set `self.DEX` (`/Game/Blueprints/Third_person/SideScrollerCharacter.DEX` _asside_scroller_character))
  (set `self.VIT` (`/Game/Blueprints/Third_person/SideScrollerCharacter.VIT` _asside_scroller_character))
  (set `self.Allocable_Points` (`/Game/Blueprints/Third_person/SideScrollerCharacter.Allocable_Points` _asside_scroller_character))
  (set `self.Date` (`KismetMathLibrary.Now`))
  (bind _returnvalue (`GameplayStatics.GetCurrentLevelName` true))
  (set `self.Cur_level_name` _returnvalue))