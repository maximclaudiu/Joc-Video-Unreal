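; Dark area entrance trigger that changes the level's SkyLight intensity as a boundary is crossed.
; Overlapping the Lower component sets the light to NewLightValue, and overlapping Upper sets it to a hard-coded intensity.
; An IsDark flag lets each change apply only when the state flips.
; Any overlapping actor triggers it, and the SkyLight is looked up by class on each overlap.
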(event `self.Upper.OnComponentBeginOverlap`
  (params (OverlappedComponent :type "PrimitiveComponent Object Reference") (OtherActor :type "Actor Object Reference") (OtherComp :type "PrimitiveComponent Object Reference") (OtherBodyIndex :type Integer) (bFromSweep :type Boolean) (SweepResult :type "HitResult Structure (by ref)"))
  (bind _returnvalue (`GameplayStatics.GetActorOfClass` "/Script/Engine.SkyLight"))
  (if (`self.IsDark?`)
    (`SkyLightComponent.SetIntensity` (`SkyLight.LightComponent` _returnvalue) 3.0)
    (set `self.IsDark?` false)))

(event `self.Lower.OnComponentBeginOverlap`
  (params (OverlappedComponent :type "PrimitiveComponent Object Reference") (OtherActor :type "Actor Object Reference") (OtherComp :type "PrimitiveComponent Object Reference") (OtherBodyIndex :type Integer) (bFromSweep :type Boolean) (SweepResult :type "HitResult Structure (by ref)"))
  (bind _returnvalue (`GameplayStatics.GetActorOfClass` "/Script/Engine.SkyLight"))
  (if (not (`self.IsDark?`))
    (`SkyLightComponent.SetIntensity` (`SkyLight.LightComponent` _returnvalue) (`self.New_Light_Value`))
    (set `self.IsDark?` true)))

(fn `UserConstructionScript`)