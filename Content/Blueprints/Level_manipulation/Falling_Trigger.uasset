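; A trigger volume that forces the side-scroller character into the Falling movement mode while it is active.
; Actor begin overlap stores the other actor and sets a falling flag, and Tick then re-applies Falling to that actor's character movement every frame if it casts to SideScrollerCharacter.
; Any end overlap on the Box component clears the flag, regardless of which actor leaves.
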(event `self.ReceiveActorBeginOverlap`
  (params (OtherActor :type "Actor Object Reference"))
  (set `self.Other Actor` OtherActor)
  (set `self.IsFalling?` true))

(event `self.ReceiveTick`
  (params (DeltaSeconds :type "Float (single-precision)"))
  (if (`self.IsFalling?`)
    (bind _asside_scroller_character (cast `/Game/Blueprints/Third_person/SideScrollerCharacter` (`self.Other Actor`)))
    (`CharacterMovementComponent.SetMovementMode` (`Character.CharacterMovement` _asside_scroller_character) "MOVE_Falling" 0)))

(event `self.Box.OnComponentEndOverlap`
  (params (OverlappedComponent :type "PrimitiveComponent Object Reference") (OtherActor :type "Actor Object Reference") (OtherComp :type "PrimitiveComponent Object Reference") (OtherBodyIndex :type Integer))
  (set `self.IsFalling?` false))

(fn `UserConstructionScript`)