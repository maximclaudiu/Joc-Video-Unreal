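; Openable treasure chest actor that rewards the player with a random amount of coins, once only.
; Its Box overlap events tell the overlapping actor to show or remove an 'F' key prompt, passing the chest as a reference.
; KeyPressed sets an Opened guard, then plays a timeline that rotates the lid.
; When the timeline finishes, it adds the coins to the Player and destroys the chest.
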(event `/Game/Blueprints/HUD/BPI_Key_Prompt.Key_pressed`
  (params (Player :type "/Game/Blueprints/Third_person/SideScrollerCharacter Object Reference"))
  (if (not (`self.Opened?`))
    (set `self.Opened?` true)
    (bind (_direction _lidposition _lidfacingrotation) (`Timeline|OpenChest`)
      (:`Update`
        (`SceneComponent.K2_SetRelativeRotation` (`self.ChestLid`) (`KismetMathLibrary.ComposeRotators` (* (struct :`Pitch` 40.0) _lidposition) (* (struct :`Yaw` 180.0) _lidfacingrotation)) false false))
      (:`Finished`
        (set `/Game/Blueprints/Third_person/SideScrollerCharacter.Coins` (+ (+ (`/Game/Blueprints/Third_person/SideScrollerCharacter.Coins` Player) (`KismetMathLibrary.RandomInteger` 100)) 100) Player)
        (`self.K2_DestroyActor`)))))

(event `self.Box.OnComponentBeginOverlap`
  (params (OverlappedComponent :type "PrimitiveComponent Object Reference") (OtherActor :type "Actor Object Reference") (OtherComp :type "PrimitiveComponent Object Reference") (OtherBodyIndex :type Integer) (bFromSweep :type Boolean) (SweepResult :type "HitResult Structure (by ref)"))
  (message `/Game/Blueprints/HUD/BPI_Key_Prompt.Create_prompt` OtherActor "Press 'F' to Open Chest" self))

(event `self.Box.OnComponentEndOverlap`
  (params (OverlappedComponent :type "PrimitiveComponent Object Reference") (OtherActor :type "Actor Object Reference") (OtherComp :type "PrimitiveComponent Object Reference") (OtherBodyIndex :type Integer))
  (message `/Game/Blueprints/HUD/BPI_Key_Prompt.Delete_prompt` OtherActor))

(fn `UserConstructionScript`)