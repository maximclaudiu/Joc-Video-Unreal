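; MarketStall is a decorative shop actor that lets the player open a shop screen while standing near it.
; It shows its name on BeginPlay, and its Box overlap creates or removes a "Press E to shop" prompt that references the stall.
; KeyPressed creates a Shop_View widget fed by the stall's InventoryComponent, switches to UI-only input with the cursor shown, and opens the SideScrollerCharacter's character info.
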(event `self.ReceiveBeginPlay`
  (`TextRenderComponent.K2_SetText` (`self.ShopName`) (`self.Name`)))

(event `/Game/Blueprints/HUD/BPI_Key_Prompt.Key_pressed`
  (params (Player :type "/Game/Blueprints/Third_person/SideScrollerCharacter Object Reference"))
  (bind _returnvalue (`GameplayStatics.GetPlayerController` 0))
  (bind _returnvalue_2 (`|CreateWidget` "/Game/Blueprints/HUD/Window_Views/Shop_View.Shop_View_C"))
  (set `/Game/Blueprints/HUD/Window_Views/Shop_View.InventoryComponent` (`self.InventoryComponent`) _returnvalue_2)
  (`UserWidget.AddToViewport` _returnvalue_2 0)
  (`WidgetBlueprintLibrary.SetInputMode_UIOnlyEx` _returnvalue _returnvalue_2)
  (set `PlayerController.bShowMouseCursor` true _returnvalue)
  (`/Game/Blueprints/Third_person/SideScrollerCharacter.OpenCharacterInfo` (cast `/Game/Blueprints/Third_person/SideScrollerCharacter` (`GameplayStatics.GetPlayerCharacter` 0) :!pure true) "i"))

(event `self.Box.OnComponentBeginOverlap`
  (params (OverlappedComponent :type "PrimitiveComponent Object Reference") (OtherActor :type "Actor Object Reference") (OtherComp :type "PrimitiveComponent Object Reference") (OtherBodyIndex :type Integer) (bFromSweep :type Boolean) (SweepResult :type "HitResult Structure (by ref)"))
  (message `/Game/Blueprints/HUD/BPI_Key_Prompt.Create_prompt` OtherActor "Press \"E\" to shop" self))

(event `self.Box.OnComponentEndOverlap`
  (params (OverlappedComponent :type "PrimitiveComponent Object Reference") (OtherActor :type "Actor Object Reference") (OtherComp :type "PrimitiveComponent Object Reference") (OtherBodyIndex :type Integer))
  (message `/Game/Blueprints/HUD/BPI_Key_Prompt.Delete_prompt` OtherActor))

(fn `UserConstructionScript`)