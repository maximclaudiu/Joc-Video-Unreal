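; Mana pickup that restores mana to a SideScrollerCharacter pawn that overlaps it.
; On overlap it adds a quarter of the character's MaxMana to Mana, then tests whether the new value plus another quarter would exceed the maximum.
; Only when that test passes does it set Mana to MaxMana and destroy itself, so otherwise the pickup stays in the level.
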(event `self.ReceiveActorBeginOverlap`
  (params (OtherActor :type "Actor Object Reference"))
  (bind _aspawn (cast `Pawn` OtherActor))
  (bind _asside_scroller_character (cast `/Game/Blueprints/Third_person/SideScrollerCharacter` _aspawn))
  (bind _maxmana (`/Game/Blueprints/Third_person/SideScrollerCharacter.MaxMana` _asside_scroller_character))
  (bind _returnvalue (+ (`/Game/Blueprints/Third_person/SideScrollerCharacter.Mana` _asside_scroller_character) (* (/ _maxmana 100.0) 25.0)))
  (set `/Game/Blueprints/Third_person/SideScrollerCharacter.Mana` _returnvalue _asside_scroller_character)
  (if (> _returnvalue _maxmana)
    (set `/Game/Blueprints/Third_person/SideScrollerCharacter.Mana` _maxmana _asside_scroller_character)
    (`self.K2_DestroyActor`)))

(fn `UserConstructionScript`)