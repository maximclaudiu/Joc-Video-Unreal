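; Enemy_BP is a base enemy NPC that takes damage and rewards the player when killed.
; DealDamage stores the attacking player and subtracts from HP, while Tick polls HP for death.
; On death it ragdolls the mesh, waits briefly, grants level-scaled experience and random coins, reports its objective ID to the player, then destroys itself.
; The Attack event is an empty stub.
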(event `self.ReceiveTick`
  (params (DeltaSeconds :type "Float (single-precision)"))
  (bind _player (`self.Player`))
  (if (<= (`self.HP`) 0.0)
    (set `self.alive` false)
    (`PrimitiveComponent.SetSimulatePhysics` (`self.Mesh`) true)
    (`KismetSystemLibrary.Delay` 1.5)
    (`/Game/Blueprints/NPC/Enemies/Damagable_BPI.Enemy_death` _player (* (`self.LVL`) 100) (`KismetMathLibrary.RandomInteger` 100))
    (`/Game/Blueprints/Third_person/SideScrollerCharacter.OnObjectiveIDCalled` _player (`self.ObjectiveID`))
    (`self.K2_DestroyActor`)))

(event `/Game/Blueprints/NPC/Enemies/Damagable_BPI.Deal_Damage`
  (params (Damage :type "Float (single-precision)") (Player :type "/Game/Blueprints/Third_person/SideScrollerCharacter Object Reference"))
  (set `self.Player` Player)
  (set `self.HP` (- (`self.HP`) Damage)))

(event `Attack`)

(fn `UserConstructionScript`)