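; Villager NPC template Blueprint that lets the side-scroller player talk to villagers and view their quests.
; When a SideScrollerCharacter overlaps its Box, it asks that character to create an 'E' to talk prompt, passing itself as the prompt's object.
; A DoOnce gate, reset on any end overlap, keeps the prompt from repeating.
; KeyPressed tells the QuestGiver, if set, to display its quest.
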(event `self.Box.OnComponentBeginOverlap`
  (params (OverlappedComponent :type "PrimitiveComponent Object Reference") (OtherActor :type "Actor Object Reference") (OtherComp :type "PrimitiveComponent Object Reference") (OtherBodyIndex :type Integer) (bFromSweep :type Boolean) (SweepResult :type "HitResult Structure (by ref)"))
  (if (== (`GameplayStatics.GetObjectClass` OtherActor) "/Game/Blueprints/Third_person/SideScrollerCharacter.SideScrollerCharacter_C")
    (`/Engine/EditorBlueprintResources/StandardMacros.DoOnce` false :!label _label
      (:`Completed`
        (message `/Game/Blueprints/HUD/BPI_Key_Prompt.Create_prompt` OtherActor "Press 'E' to talk" self)))))

(event `self.Box.OnComponentEndOverlap`
  (params (OverlappedComponent :type "PrimitiveComponent Object Reference") (OtherActor :type "Actor Object Reference") (OtherComp :type "PrimitiveComponent Object Reference") (OtherBodyIndex :type Integer))
  (goto _label :!via `Reset`))

(event `/Game/Blueprints/HUD/BPI_Key_Prompt.Key_pressed`
  (params (Player :type "/Game/Blueprints/Third_person/SideScrollerCharacter Object Reference"))
  (if (`self.QuestGiver?`)
    (`/Game/Blueprints/Quests/QuestGiver.DisplayTheQuest` (`self.QuestGiver`))))

(fn `UserConstructionScript`)