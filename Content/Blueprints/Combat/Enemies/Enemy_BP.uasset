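; Enemy Blueprint for combat that takes damage, dies and rewards the player.
; DealDamage stores the attacking player and subtracts from HP.
; Tick polls HP; at zero or below it enables mesh physics, waits briefly, awards level-scaled experience and random coins through the player's EnemyDeath, then destroys the actor.
; The Attack event is an empty stub.
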(event `self.ReceiveTick`
  (params (DeltaSeconds :type "Float (single-precision)"))
  (if (<= (`self.HP`) 0.0)
    (set `self.alive` false)
    (`PrimitiveComponent.SetSimulatePhysics` (`self.Mesh`) true)
    (`KismetSystemLibrary.Delay` 1.5)
    (`/Game/Blueprints/Combat/Damagable_BPI.Enemy_death` (`self.Player`) (* (`self.LVL`) 100) (`KismetMathLibrary.RandomInteger` 100))
    (`self.K2_DestroyActor`)))

(event `/Game/Blueprints/Combat/Damagable_BPI.Deal_Damage`
  (params (Damage :type "Float (single-precision)") (Player :type "/Game/Blueprints/Third_person/SideScrollerCharacter Object Reference"))
  (set `self.Player` Player)
  (set `self.HP` (- (`self.HP`) Damage)))

(event `Attack`
  (params (seeTarget :type Boolean)))

(fn `UserConstructionScript`)