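; Save file Blueprint that restores saved quest state into a QuestLog.
; LoadQuest re-adds each active quest to the log, then copies its current stage and objective progress from the QuestProgress map.
; It then overwrites the log's completed and active quest lists with the saved ones.
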(fn `Load Quest`
  (params (QuestLog :type "/Game/Blueprints/Quests/QuestLogComponent Object Reference"))
  (for _array_element (`self.CurrentActiveQuest`)
    (bind _returnvalue (`/Game/Blueprints/Quests/QuestLogComponent.AddNewQuest` QuestLog _array_element))
    (bind (_progress _currentstage) (break `/Game/Blueprints/Quests/FQuestSave` (`BlueprintMapLibrary.Map_Find` (`self.QuestProgress`) _array_element)))
    (set `/Game/Blueprints/Quests/Quest_Base_BP.CurrentStage` _currentstage _returnvalue)
    (set `/Game/Blueprints/Quests/Quest_Base_BP.CurrentObjectiveProgres` _progress _returnvalue))
  (set `/Game/Blueprints/Quests/QuestLogComponent.CompletedQuests` (`self.CompletedQuests`) QuestLog)
  (set `/Game/Blueprints/Quests/QuestLogComponent.CurrentActiveQuests` (`self.CurrentActiveQuest`) QuestLog))