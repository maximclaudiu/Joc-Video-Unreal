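; Inventory component that holds a fixed-size array of item slots and handles adding, removing, dropping and consuming items.
; Adding works one unit at a time, filling non-full stacks up to the ItemData table's max size before claiming empty slots.
; Dropping spawns the item's class ahead of the player with its quantity; using spawns a consumable to call Consume.
; Removal and use refresh the Inventory_View widget.
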(event `self.ReceiveBeginPlay`
  (`KismetArrayLibrary.Array_Resize` (`self.Inventory`) (`self.NumberOfSlots`)))

(fn `AddToExistingNotFullSlot`
  (params (TargetArray :type "Array of /Game/Blueprints/InventorySystem/InventorySlotSrtucture Structure (by ref)") (Index :type Integer))
  (bind (_output_itemid _output_quantity) (break `/Game/Blueprints/InventorySystem/InventorySlotSrtucture` (`|GetArrayItem` (`self.Inventory`) Index)))
  (`KismetArrayLibrary.Array_Set` TargetArray Index (make `/Game/Blueprints/InventorySystem/InventorySlotSrtucture` _output_itemid (+ _output_quantity 1))))

(fn `AddToInventory`
  (params (ItemID :type Name) (Quantity :type Integer))
  (returns (Success :type Boolean) (RemainignQuantity :type Integer))
  (locals (LocalQuantityRemaining :type Integer) (FailedToAdd :type Boolean))
  (bind _localquantityremaining (`local.LocalQuantityRemaining`))
  (bind _inventory (`self.Inventory`))
  (bind _output_get (set `local.LocalQuantityRemaining` Quantity))
  (while (and (> _output_get 0) (not (`local.FailedToAdd`)))
    (bind (_id _success) (`self.FindSlot` (`local.ItemID`)))
    (if _success
      (`self.AddToExistingNotFullSlot` _inventory _id)
      (`/Engine/EditorBlueprintResources/StandardMacros.DecrementInt` _localquantityremaining)
      (else
        (bind _failedtocreatenewstack (`self.CreateNewItemStack` _inventory (`local.ItemID`)))
        (`/Engine/EditorBlueprintResources/StandardMacros.DecrementInt` _localquantityremaining
          (:`  `
            (set `local.FailedToAdd` _failedtocreatenewstack))))))
  (return (not (`local.FailedToAdd`)) (`local.LocalQuantityRemaining`)))

(fn `CreateNewItemStack`
  (params (Array :type "Array of /Game/Blueprints/InventorySystem/InventorySlotSrtucture Structure") (ItemID :type Name))
  (returns (FailedToCreateNewStack :type Boolean))
  (for (_array_element _array_index) Array
    (if (== (`.Quantity_6_9E5E27B4486661A7EA22D0B9BF45EE17` (break `/Game/Blueprints/InventorySystem/InventorySlotSrtucture` _array_element)) 0)
      (`KismetArrayLibrary.Array_Set` (`self.Inventory`) _array_index (make `/Game/Blueprints/InventorySystem/InventorySlotSrtucture` ItemID 1))
      (return false)))
  (return true))

(fn `FindSlot`
  (params (ItemID :type Name))
  (returns (ID :type Integer) (Success :type Boolean))
  (bind _itemid (`local.ItemID`))
  (for (_array_element _array_index) (`self.Inventory`)
    (bind (_itemid_2 _quantity) (break `/Game/Blueprints/InventorySystem/InventorySlotSrtucture` _array_element))
    (if (== _itemid_2 _itemid)
      (bind _returnvalue (`|GetDataTableRow` "/Game/Blueprints/InventorySystem/ItemData.ItemData" _itemid)
        (:`then`
          (if (< _quantity (`.MaxStackSize_12_A3D5D4444A760D916D59C5810791CB9D` (break `/Game/Blueprints/InventorySystem/ItemStructure` _returnvalue)))
            (return _array_index true))))))
  (return -1 false))

(fn `RemoveFromInventory`
  (params (Index :type Integer) (Drop :type Boolean))
  (bind _returnvalue (`GameplayStatics.GetPlayerCharacter` 0))
  (bind _inventory (`self.Inventory`))
  (bind (_output_itemid _output_quantity) (break `/Game/Blueprints/InventorySystem/InventorySlotSrtucture` (`|GetArrayItem` _inventory Index)))
  (bind _output (`|GetArrayItem` _inventory Index))
  (if Drop
    (bind _returnvalue_2 (`|GetDataTableRow` "/Game/Blueprints/InventorySystem/ItemData.ItemData" _output_itemid)
      (:`then`
        (bind _returnvalue_3 (`|SpawnActorFromClass` (`.Class_17_4BBCED80412654587A1F3C8FDA0EE7DD` (break `/Game/Blueprints/InventorySystem/ItemStructure` _returnvalue_2)) (`KismetMathLibrary.MakeTransform` (+ (`SceneComponent.K2_GetComponentLocation` (`Character.CapsuleComponent` _returnvalue)) (* (`Actor.GetActorForwardVector` _returnvalue) 100))) "Undefined" "OverrideRootScale" null null))
        (set `/Game/Blueprints/InventorySystem/ItemDataComponent.Quantity` _output_quantity (`/Game/Blueprints/InventorySystem/Item.ItemDataComponent` _returnvalue_3))
        (setmembers `/Game/Blueprints/InventorySystem/InventorySlotSrtucture` :`StructRef` _output :`ItemID` "None" :`Quantity` 0)
        (bind _foundwidgets (`WidgetBlueprintLibrary.GetAllWidgetsOfClass` "/Game/Blueprints/HUD/Window_Views/Inventory_View.Inventory_View_C" false))
        (for _array_element _foundwidgets
          (`/Game/Blueprints/HUD/Window_Views/Inventory_View.UpdateInventory` _array_element)
          (break))))
    (else
      (setmembers `/Game/Blueprints/InventorySystem/InventorySlotSrtucture` :`StructRef` _output :`ItemID` "None" :`Quantity` 0)
      (bind _foundwidgets_2 (`WidgetBlueprintLibrary.GetAllWidgetsOfClass` "/Game/Blueprints/HUD/Window_Views/Inventory_View.Inventory_View_C" false))
      (for _array_element_2 _foundwidgets_2
        (`/Game/Blueprints/HUD/Window_Views/Inventory_View.UpdateInventory` _array_element_2)
        (break)))))

(fn `UseItem`
  (params (Index :type Integer) (`RealUse?` :type Boolean))
  (bind _output (`|GetArrayItem` (`self.Inventory`) Index))
  (bind (_itemid _quantity) (break `/Game/Blueprints/InventorySystem/InventorySlotSrtucture` _output))
  (bind _returnvalue (`|GetDataTableRow` "/Game/Blueprints/InventorySystem/ItemData.ItemData" _itemid)
    (:`then`
      (bind (_name _maxstacksize _class _thumbnail _consumable) (break `/Game/Blueprints/InventorySystem/ItemStructure` _returnvalue))
      (if _consumable
        (bind _returnvalue_2 (`|SpawnActorFromClass` _class (`KismetMathLibrary.MakeTransform` (0.0 0.0 0.0)) "Undefined" "OverrideRootScale" null null))
        (`/Game/Blueprints/InventorySystem/Item.Consume` _returnvalue_2 `RealUse?`)
        (if (== 1 _quantity)
          (`self.RemoveFromInventory` (`local.Index`))
          (else
            (setmembers `/Game/Blueprints/InventorySystem/InventorySlotSrtucture` :`StructRef` _output :`ItemID` _itemid :`Quantity` (- _quantity 1))))
        (bind _foundwidgets (`WidgetBlueprintLibrary.GetAllWidgetsOfClass` "/Game/Blueprints/HUD/Window_Views/Inventory_View.Inventory_View_C" false))
        (for _array_element _foundwidgets
          (`/Game/Blueprints/HUD/Window_Views/Inventory_View.UpdateInventory` _array_element)
          (break))))))