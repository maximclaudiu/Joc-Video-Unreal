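; Base pickup item actor for the inventory system, which the player collects with a key press.
; Its collision box shows an 'E' prompt on overlapping actors that implement BPI_Key_Prompt and requests its removal when overlap ends.
; KeyPressed passes the ItemDataComponent's row ID and quantity to the player's InventoryComponent, keeps any remainder and destroys the actor at zero.
; The Consume event is an empty stub.
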(event `self.collisionBox.OnComponentBeginOverlap`
  (params (OverlappedComponent :type "PrimitiveComponent Object Reference") (OtherActor :type "Actor Object Reference") (OtherComp :type "PrimitiveComponent Object Reference") (OtherBodyIndex :type Integer) (bFromSweep :type Boolean) (SweepResult :type "HitResult Structure (by ref)"))
  (if (`KismetSystemLibrary.DoesImplementInterface` OtherActor "/Game/Blueprints/HUD/BPI_Key_Prompt.BPI_Key_Prompt_C")
    (message `/Game/Blueprints/HUD/BPI_Key_Prompt.Create_prompt` OtherActor "Press 'E' to pick up item" self)))

(event `self.collisionBox.OnComponentEndOverlap`
  (params (OverlappedComponent :type "PrimitiveComponent Object Reference") (OtherActor :type "Actor Object Reference") (OtherComp :type "PrimitiveComponent Object Reference") (OtherBodyIndex :type Integer))
  (message `/Game/Blueprints/HUD/BPI_Key_Prompt.Delete_prompt` OtherActor))

(event `/Game/Blueprints/HUD/BPI_Key_Prompt.Key_pressed`
  (params (Player :type "/Game/Blueprints/Third_person/SideScrollerCharacter Object Reference"))
  (bind _itemdatacomponent (`self.ItemDataComponent`))
  (bind (_itemid_datatable _itemid_rowname) (break `DataTableRowHandle` (`/Game/Blueprints/InventorySystem/ItemDataComponent.ItemID` _itemdatacomponent)))
  (bind (_success _remainignquantity) (`/Game/Blueprints/InventorySystem/InventoryComponent.AddToInventory` (`/Game/Blueprints/Third_person/SideScrollerCharacter.InventoryComponent` Player) _itemid_rowname (`/Game/Blueprints/InventorySystem/ItemDataComponent.Quantity` _itemdatacomponent)))
  (if _success
    (bind _output_get (set `/Game/Blueprints/InventorySystem/ItemDataComponent.Quantity` _remainignquantity _itemdatacomponent))
    (if (== _output_get 0)
      (`self.K2_DestroyActor`))))

(event `Consume`
  (params (RealUse :type Boolean)))

(fn `UserConstructionScript`)